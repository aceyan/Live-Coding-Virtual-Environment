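; Ray-marching pickup Blueprint that supplies a second shape (P2) and its combine settings to the mesh's materials.
; Each Tick runs the parent logic, takes the actor's location as the P2 position, then pushes it with operation type, operand index, smoothing and geometry type as material parameters.
; A switch on geometry type pushes only that primitive's dimensions, covering shapes from sphere to capsule.
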(event EventBeginPlay
  (|CallParentFunction) ; This node is disabled and will not be called.\nDrag off pins to build functionality.
)

(event Collision|EventActorBeginOverlap
  (params (OtherActor :type Actor%20Object%20Reference))
  (|CallParentFunction OtherActor) ; This node is disabled and will not be called.\nDrag off pins to build functionality.
)

(event EventTick
  (params (DeltaSeconds :type Float%20%28single-precision%29))
  (bind _staticmeshcomponent (Variables|Default|GetStaticMeshComponent))
  (bind _staticmeshcomponent_2 (Variables|Default|GetStaticMeshComponent))
  (|CallParentFunction DeltaSeconds)
  ;[1 1 1] TODO
  (Variables|RayMarchingCombinable2|SetP2ObjectPosition (Transformation|GetActorLocation))
  ;[1 1 1] common
  (Rendering|Material|SetScalarParameterValueonMaterials (Variables|Default|GetStaticMeshComponent) "OperationType" (Math|Conversions|ToFloat(Integer) (Variables|RayMarchingCombinable2|GetOperationType)))
  (Rendering|Material|SetScalarParameterValueonMaterials (Variables|Default|GetStaticMeshComponent) "OperandIndex" (Math|Conversions|ToFloat(Integer) (Variables|RayMarchingCombinable2|GetOperandIndex)))
  (Rendering|Material|SetScalarParameterValueonMaterials (Variables|Default|GetStaticMeshComponent) "Smooth" (Variables|RayMarchingCombinable2|GetSmooth))
  (Rendering|Material|SetScalarParameterValueonMaterials (Variables|Default|GetStaticMeshComponent) "P2GeometryType" (Math|Conversions|ToFloat(Integer) (Variables|RayMarchingCombinable2|GetP2GeometryType)))
  (Rendering|Material|SetVectorParameterValueonMaterials (Variables|Default|GetStaticMeshComponent) "P2ObjectPosition" (Variables|RayMarchingCombinable2|GetP2ObjectPosition))
  (switch Utilities|FlowControl|Switch|SwitchonRayMarchingSingleShapeTypes (Utilities|Enum|ByteToEnumRayMarchingSingleShapeTypes (Math|Conversions|ToByte(Integer) (Variables|RayMarchingCombinable2|GetP2GeometryType)))
    (:NewEnumerator0
      ;[1 1 1] Sphere
      (Rendering|Material|SetScalarParameterValueonMaterials (Variables|Default|GetStaticMeshComponent) "P2SphereRadius" (Variables|RayMarchingCombinable2|GetP2SphereRadius)))
    (:NewEnumerator1
      ;[1 1 1] Box
      (Rendering|Material|SetVectorParameterValueonMaterials (Variables|Default|GetStaticMeshComponent) "P2BoxDimension" (Variables|RayMarchingCombinable2|GetP2BoxDimension)))
    (:NewEnumerator2
      ;[1 1 1] RoundBox
      (Rendering|Material|SetScalarParameterValueonMaterials _staticmeshcomponent "P2BoxRound" (Variables|RayMarchingCombinable2|GetP2BoxRound))
      (Rendering|Material|SetVectorParameterValueonMaterials _staticmeshcomponent "P2BoxDimension" (Variables|RayMarchingCombinable2|GetP2BoxDimension)))
    (:NewEnumerator3
      ;[1 1 1] Torus
      (Rendering|Material|SetVectorParameterValueonMaterials (Variables|Default|GetStaticMeshComponent) "P2TorusDimension" (Variables|RayMarchingCombinable2|GetP2TorusDimension)))
    (:NewEnumerator4
      ;[1 1 1] Link
      (Rendering|Material|SetScalarParameterValueonMaterials (Variables|Default|GetStaticMeshComponent) "P2LinkLength" (Variables|RayMarchingCombinable2|GetP2LinkLength))
      (Rendering|Material|SetScalarParameterValueonMaterials (Variables|Default|GetStaticMeshComponent) "P2LinkRadius1" (Variables|RayMarchingCombinable2|GetP2LinkRadius1))
      (Rendering|Material|SetScalarParameterValueonMaterials (Variables|Default|GetStaticMeshComponent) "P2LinkRadius2" (Variables|RayMarchingCombinable2|GetP2LinkRadius2)))
    (:NewEnumerator5
      ;[1 1 1] Cylinder
      (Rendering|Material|SetScalarParameterValueonMaterials (Variables|Default|GetStaticMeshComponent) "P2CylinderRadius" (Variables|RayMarchingCombinable2|GetP2CylinderRadius))
      (Rendering|Material|SetScalarParameterValueonMaterials (Variables|Default|GetStaticMeshComponent) "P2CylinderLength" (Variables|RayMarchingCombinable2|GetP2CylinderLength)))
    (:NewEnumerator6
      ;[1 1 1] Cone
      (Rendering|Material|SetVectorParameterValueonMaterials _staticmeshcomponent_2 "P2ConeAngle" (Variables|RayMarchingCombinable2|GetP2ConeAngle))
      (Rendering|Material|SetScalarParameterValueonMaterials _staticmeshcomponent_2 "P2ConeLength" (Variables|RayMarchingCombinable2|GetP2ConeLength)))
    (:NewEnumerator7
      ;[1 1 1] Capsule
      (Rendering|Material|SetVectorParameterValueonMaterials (Variables|Default|GetStaticMeshComponent) "P2CapsuleDimension1" (Variables|RayMarchingCombinable2|GetP2CapsuleDimension1))
      (Rendering|Material|SetVectorParameterValueonMaterials (Variables|Default|GetStaticMeshComponent) "P2CapsuleDimension2" (Variables|RayMarchingCombinable2|GetP2CapsuleDimension2))
      (Rendering|Material|SetScalarParameterValueonMaterials (Variables|Default|GetStaticMeshComponent) "P2CapsuleRadius" (Variables|RayMarchingCombinable2|GetP2CapsuleRadius)))))

(fn ConstructionScript
  (|CallParentFunction))