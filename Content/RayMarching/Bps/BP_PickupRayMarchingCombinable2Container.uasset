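; Container actor that spawns two ray-marched combinable pickups at its transform, both tagged "Apple", with the second given a different geometry type.
; Each Tick it pushes its shared operation type, smoothing and surface color to both, along with each one's operand index.
; It also cross-feeds each pickup the other's mesh location and geometry data, so both hold the two operands of the combine operation.
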(event EventBeginPlay
  (Utilities|FlowControl|Sequence
    (:then_0
      (bind _returnvalue (Game|SpawnActorfromClass :Class "/Game/RayMarching/Bps/BP_PickupRayMarchingCombinable2.BP_PickupRayMarchingCombinable2_C" :SpawnTransform (Transformation|GetActorTransform) :CollisionHandlingOverride "Undefined" :SurfaceColor (Variables|RayMarchingCombinable2Container|GetSurfaceColor) :Instigator 0))
      (Utilities|Array|Add (Variables|/Script/Engine.Actor|GetTags _returnvalue) (Utilities|Name|MakeLiteralName "Apple"))
      (Variables|RayMarchingCombinable2Container|Setobject1 _returnvalue))
    (:then_1
      (bind _returnvalue_2 (Game|SpawnActorfromClass "/Game/RayMarching/Bps/BP_PickupRayMarchingCombinable2.BP_PickupRayMarchingCombinable2_C" (Transformation|GetActorTransform) "Undefined" 0 (Variables|RayMarchingCombinable2Container|GetSurfaceColor) (Utilities|Struct|MakeRayMarchingGeometryData 1 2e+01 "15.000000,15.000000,15.000000" 5.0 "15.000000,8.000000,0.000000" 7.0 12.0 6.0 12.0 15.0 "3.000000,6.000000,0.000000" 4e+01 "0.000000,15.000000,0.000000" "0.000000,-15.000000,0.000000" 15.0) 0))
      (Utilities|Array|Add (Variables|/Script/Engine.Actor|GetTags _returnvalue_2) (Utilities|Name|MakeLiteralName "Apple"))
      (Variables|RayMarchingCombinable2Container|Setobject2 _returnvalue_2))))

(event Collision|EventActorBeginOverlap
  (params (OtherActor :type Actor%20Object%20Reference)))

(event EventTick
  (params (DeltaSeconds :type Float%20%28single-precision%29))
  (bind _object1 (Variables|RayMarchingCombinable2Container|Getobject1))
  (bind _object2 (Variables|RayMarchingCombinable2Container|Getobject2))
  (bind _object1_2 (Variables|RayMarchingCombinable2Container|Getobject1))
  (bind _object2_2 (Variables|RayMarchingCombinable2Container|Getobject2))
  (bind _object1_3 (Variables|RayMarchingCombinable2Container|Getobject1))
  (bind _object2_3 (Variables|RayMarchingCombinable2Container|Getobject2))
  (Utilities|FlowControl|Sequence
    (:then_0
      ;[1 1 1] Basic
      (Variables|/Game/RayMarching/Bps/BP_PickupRayMarchingCombinable2.BP_PickupRayMarchingCombinable2_C|SetOperationType _object1 (Variables|RayMarchingCombinable2Container|GetOperationType))
      (Variables|/Game/RayMarching/Bps/BP_PickupRayMarchingCombinable2.BP_PickupRayMarchingCombinable2_C|SetSmooth _object1 (Variables|RayMarchingCombinable2Container|GetSmooth))
      (Variables|/Game/RayMarching/Bps/BP_PickupRayMarchingSingleShape.BP_PickupRayMarchingSingleShape_C|SetSurfaceColor _object1 (Variables|RayMarchingCombinable2Container|GetSurfaceColor))
      (Variables|/Game/RayMarching/Bps/BP_PickupRayMarchingCombinable2.BP_PickupRayMarchingCombinable2_C|SetOperandIndex _object1 0)
      ;[1 1 1] Geometry data
      (Variables|/Game/RayMarching/Bps/BP_PickupRayMarchingCombinable2.BP_PickupRayMarchingCombinable2_C|SetP2ObjectPosition _object1_2 (Transformation|GetWorldLocation (Variables|/Script/Engine.StaticMeshActor|GetStaticMeshComponent _object2)))
      (Variables|/Game/RayMarching/Bps/BP_PickupRayMarchingCombinable2.BP_PickupRayMarchingCombinable2_C|SetP2GeometyData _object1_2 (Variables|/Game/RayMarching/Bps/BP_PickupRayMarchingSingleShape.BP_PickupRayMarchingSingleShape_C|GetGeometryData _object2)))
    (:then_1
      ;[1 1 1] Basic
      (Variables|/Game/RayMarching/Bps/BP_PickupRayMarchingCombinable2.BP_PickupRayMarchingCombinable2_C|SetOperationType _object2_2 (Variables|RayMarchingCombinable2Container|GetOperationType))
      (Variables|/Game/RayMarching/Bps/BP_PickupRayMarchingCombinable2.BP_PickupRayMarchingCombinable2_C|SetSmooth _object2_2 (Variables|RayMarchingCombinable2Container|GetSmooth))
      (Variables|/Game/RayMarching/Bps/BP_PickupRayMarchingSingleShape.BP_PickupRayMarchingSingleShape_C|SetSurfaceColor _object2_2 (Variables|RayMarchingCombinable2Container|GetSurfaceColor))
      (Variables|/Game/RayMarching/Bps/BP_PickupRayMarchingCombinable2.BP_PickupRayMarchingCombinable2_C|SetOperandIndex _object2_2 1)
      ;[1 1 1] Geometry data
      (Variables|/Game/RayMarching/Bps/BP_PickupRayMarchingCombinable2.BP_PickupRayMarchingCombinable2_C|SetP2ObjectPosition _object2_3 (Transformation|GetWorldLocation (Variables|/Script/Engine.StaticMeshActor|GetStaticMeshComponent _object1_3)))
      (Variables|/Game/RayMarching/Bps/BP_PickupRayMarchingCombinable2.BP_PickupRayMarchingCombinable2_C|SetP2GeometyData _object2_3 (Variables|/Game/RayMarching/Bps/BP_PickupRayMarchingSingleShape.BP_PickupRayMarchingSingleShape_C|GetGeometryData _object1_3)))))

(fn ConstructionScript)