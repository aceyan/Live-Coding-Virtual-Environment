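; Pickup fractal actor that displays a fractal through a material on its static mesh, with adjustable radius, iteration count, power and color.
; Every Tick pushes these variables into the mesh materials as scalar and vector parameters.
; It also rescales the root component uniformly to the sphere's diameter divided by 100, keeping actor size in step with the radius sent to the shader.
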(event EventBeginPlay
  (|CallParentFunction) ; This node is disabled and will not be called.\nDrag off pins to build functionality.
)

(event Collision|EventActorBeginOverlap
  (params (OtherActor :type Actor%20Object%20Reference))
  (|CallParentFunction OtherActor) ; This node is disabled and will not be called.\nDrag off pins to build functionality.
)

(event EventTick
  (params (DeltaSeconds :type Float%20%28single-precision%29))
  (bind _sphereradius (Variables|Fractal|GetSphereRadius))
  (bind _returnvalue (* 2 _sphereradius))
  (bind _returnvalue_2 (/ _returnvalue 1e+02))
  (|CallParentFunction DeltaSeconds)
  (Rendering|Material|SetScalarParameterValueonMaterials (Variables|Default|GetStaticMeshComponent) "SphereRadius" (Variables|Fractal|GetSphereRadius))
  (Rendering|Material|SetScalarParameterValueonMaterials (Variables|Default|GetStaticMeshComponent) "IterationNum" (Variables|Fractal|GetIterationNum))
  (Rendering|Material|SetScalarParameterValueonMaterials (Variables|Default|GetStaticMeshComponent) "PowerNum" (Variables|Fractal|GetPowerNum))
  (Rendering|Material|SetVectorParameterValueonMaterials (Variables|Default|GetStaticMeshComponent) "color" (Variables|Fractal|GetFractalColor))
  (Transformation|SetRelativeScale3D (Variables|Transformation|GetRootComponent) (Math|Vector|MakeVector _returnvalue_2 _returnvalue_2 _returnvalue_2)))

(fn ConstructionScript
  (|CallParentFunction))