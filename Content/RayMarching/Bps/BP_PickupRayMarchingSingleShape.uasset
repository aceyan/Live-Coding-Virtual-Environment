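; Pickup actor that displays a single ray-marched primitive, such as a sphere, box, torus or capsule, through its static mesh's materials.
; Every Tick pushes the shape type, march settings, color and that shape's GeometryData dimensions into material parameters.
; It also uniformly rescales the root from those dimensions, apparently so the proxy mesh encloses the ray-marched shape.
; BeginPlay and construction only call the parent.
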(event EventBeginPlay
  (|CallParentFunction))

(event Collision|EventActorBeginOverlap
  (params (OtherActor :type Actor%20Object%20Reference))
  (|CallParentFunction OtherActor) ; This node is disabled and will not be called.\nDrag off pins to build functionality.
)

(event EventTick
  (params (DeltaSeconds :type Float%20%28single-precision%29))
  (bind _geometrydata (Variables|RayMarchingSingleShape|GetGeometryData))
  (bind _staticmeshcomponent (Variables|Default|GetStaticMeshComponent))
  (bind _geometrydata_2 (Variables|RayMarchingSingleShape|GetGeometryData))
  (bind _staticmeshcomponent_2 (Variables|Default|GetStaticMeshComponent))
  (bind (_geometrytype _sphereradius _boxdimension _boxround _torusdimension _linklength _linkradius1 _linkradius2 _cylinderradius _cylinderlength _coneangle _conelength _capsuledimension1 _capsuledimension2 _capsuleradius) (Utilities|Struct|BreakRayMarchingGeometryData _geometrydata))
  (bind (_geometrytype_2 _sphereradius_2 _boxdimension_2 _boxround_2 _torusdimension_2 _linklength_2 _linkradius1_2 _linkradius2_2 _cylinderradius_2 _cylinderlength_2 _coneangle_2 _conelength_2 _capsuledimension1_2 _capsuledimension2_2 _capsuleradius_2) (Utilities|Struct|BreakRayMarchingGeometryData _geometrydata_2))
  (|CallParentFunction DeltaSeconds)
  ;[1 1 1] common
  (Rendering|Material|SetScalarParameterValueonMaterials (Variables|Default|GetStaticMeshComponent) "GeometryType" (Math|Conversions|ToFloat(Integer) (.GeometryType (Utilities|Struct|BreakRayMarchingGeometryData (Variables|RayMarchingSingleShape|GetGeometryData)))))
  (Rendering|Material|SetScalarParameterValueonMaterials (Variables|Default|GetStaticMeshComponent) "MaxSteps" (Variables|RayMarchingSingleShape|GetMaxSteps))
  (Rendering|Material|SetScalarParameterValueonMaterials (Variables|Default|GetStaticMeshComponent) "DisThreadhold" (Variables|RayMarchingSingleShape|GetDisThreadhold))
  (Rendering|Material|SetVectorParameterValueonMaterials (Variables|Default|GetStaticMeshComponent) "SurfaceColor" (Variables|RayMarchingSingleShape|GetSurfaceColor))
  (switch Utilities|FlowControl|Switch|SwitchonRayMarchingSingleShapeTypes (Utilities|Enum|ByteToEnumRayMarchingSingleShapeTypes (Math|Conversions|ToByte(Integer) _geometrytype_2))
    (:NewEnumerator0
      ;[1 1 1] Sphere
      (Rendering|Material|SetScalarParameterValueonMaterials (Variables|Default|GetStaticMeshComponent) "SphereRadius" _sphereradius_2)
      ;[1 1 1] reset scale
      (Transformation|SetRelativeScale3D (Variables|Transformation|GetRootComponent) (* "1.000000,1.000000,1.000000" (/ _sphereradius 45.0))))
    (:NewEnumerator1
      ;[1 1 1] Box
      (Rendering|Material|SetVectorParameterValueonMaterials (Variables|Default|GetStaticMeshComponent) "BoxDimension" _boxdimension_2)
      ;[1 1 1] reset scale
      (Transformation|SetRelativeScale3D (Variables|Transformation|GetRootComponent) (* "1.000000,1.000000,1.000000" (/ (* (Math|Vector|GetMaxElement _boxdimension) 1.42) 4e+01))))
    (:NewEnumerator2
      ;[1 1 1] RoundBox
      (Rendering|Material|SetScalarParameterValueonMaterials _staticmeshcomponent "BoxRound" _boxround_2)
      (Rendering|Material|SetVectorParameterValueonMaterials _staticmeshcomponent "BoxDimension" _boxdimension_2)
      ;[1 1 1] reset scale
      (Transformation|SetRelativeScale3D (Variables|Transformation|GetRootComponent) (* "1.000000,1.000000,1.000000" (/ (* (+ (Math|Vector|GetMaxElement _boxdimension) _boxround) 1.42) 4e+01))))
    (:NewEnumerator3
      ;[1 1 1] Torus
      (Rendering|Material|SetVectorParameterValueonMaterials (Variables|Default|GetStaticMeshComponent) "TorusDimension" _torusdimension_2)
      ;[1 1 1] reset scale
      (Transformation|SetRelativeScale3D (Variables|Transformation|GetRootComponent) (* "1.000000,1.000000,1.000000" (/ (+ (.x _torusdimension) (.y _torusdimension)) 4e+01))))
    (:NewEnumerator4
      ;[1 1 1] Link
      (Rendering|Material|SetScalarParameterValueonMaterials (Variables|Default|GetStaticMeshComponent) "LinkLength" _linklength_2)
      (Rendering|Material|SetScalarParameterValueonMaterials (Variables|Default|GetStaticMeshComponent) "LinkRadius1" _linkradius1_2)
      (Rendering|Material|SetScalarParameterValueonMaterials (Variables|Default|GetStaticMeshComponent) "LinkRadius2" _linkradius2_2)
      ;[1 1 1] reset scale
      (Transformation|SetRelativeScale3D (Variables|Transformation|GetRootComponent) (* "1.000000,1.000000,1.000000" (/ (+ _linklength _linkradius1 _linkradius2) 45.0))))
    (:NewEnumerator5
      ;[1 1 1] Cylinder
      (Rendering|Material|SetScalarParameterValueonMaterials (Variables|Default|GetStaticMeshComponent) "CylinderRadius" _cylinderradius_2)
      (Rendering|Material|SetScalarParameterValueonMaterials (Variables|Default|GetStaticMeshComponent) "CylinderLength" _cylinderlength_2)
      ;[1 1 1] reset scale
      (Transformation|SetRelativeScale3D (Variables|Transformation|GetRootComponent) (* "1.000000,1.000000,1.000000" (/ (Math|Float|Max(Float) (* _cylinderlength 1.42) (* _cylinderradius 1.42)) 45.0))))
    (:NewEnumerator6
      ;[1 1 1] Cone
      (Rendering|Material|SetVectorParameterValueonMaterials _staticmeshcomponent_2 "ConeAngle" _coneangle_2)
      (Rendering|Material|SetScalarParameterValueonMaterials _staticmeshcomponent_2 "ConeLength" _conelength_2)
      ;[1 1 1] reset scale
      (Transformation|SetRelativeScale3D (Variables|Transformation|GetRootComponent) (* "1.000000,1.000000,1.000000" (/ (Math|Float|Sqrt (+ (Math|Float|Power _conelength 2.0) (Math|Float|Power (* _conelength (/ (.x _coneangle) (.y _coneangle))) 2.0))) 45.0))))
    (:NewEnumerator7
      ;[1 1 1] Capsule
      (Rendering|Material|SetVectorParameterValueonMaterials (Variables|Default|GetStaticMeshComponent) "CapsuleDimension1" _capsuledimension1_2)
      (Rendering|Material|SetVectorParameterValueonMaterials (Variables|Default|GetStaticMeshComponent) "CapsuleDimension2" _capsuledimension2_2)
      (Rendering|Material|SetScalarParameterValueonMaterials (Variables|Default|GetStaticMeshComponent) "CapsuleRadius" _capsuleradius_2)
      ;[1 1 1] reset scale
      (Transformation|SetRelativeScale3D (Variables|Transformation|GetRootComponent) (* "1.000000,1.000000,1.000000" (/ (+ (/ (+ (Math|Float|Absolute(Float) (.y _capsuledimension1)) (Math|Float|Absolute(Float) (.y _capsuledimension2))) 2.0) _capsuleradius) 45.0))))))

(fn ConstructionScript
  (|CallParentFunction))