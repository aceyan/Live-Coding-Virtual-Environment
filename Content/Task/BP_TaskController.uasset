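; Task controller that walks the player through an ordered list of tasks and steps defined in TaskAssetData.
; On BeginPlay it binds to the FPSPawn's LeftController creation, editing and query events, plus the pawn's tag updates.
; Each handler advances only if the current step's type matches that action; event parameters are ignored.
; UpdateTaskStep moves to the next step or task, then fires CallTaskUpdate; progress is printed for debugging.
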(event Custom|OnAdjustSmallFlocking
  (CallBack|OnAdjustSmallFlockingFunc))

(event Custom|OnCreateRayMarching
  (params (GeometryType :type RayMarchingSingleShapeTypes%20Enum :default "NewEnumerator0") (count :type Integer))
  (CallBack|OnCreateRayMarchingFunc GeometryType count))

(event Custom|OnChangeShapeRayMarching
  (params (GeometryType :type RayMarchingSingleShapeTypes%20Enum :default "NewEnumerator0"))
  (CallBack|OnChangeShapeRayMarchingFunc GeometryType))

(event Custom|OnChangeColorMeshBased
  (params (colorVector :type Vector))
  (CallBack|OnChangeColorMeshBasedFunc colorVector))

(event Custom|OnChangeColorRayMarching
  (params (color :type Vector))
  (CallBack|OnChangeColorRayMarchingFunc color))

(event Custom|OnScaleRayMarching
  (CallBack|OnScaleRayMarchingFunc))

(event Custom|OnScaleCube
  (CallBack|OnScaleCubeFunc))

(event Custom|OnCreateFractal
  (CallBack|OnCreateFractalFunc))

(event Custom|OnTagsUpdate
  (CallBack|OnTagsUpdateFunc))

(event Custom|OnQuerySuccess
  (CallBack|OnQuerySuccessFunc))

(event Custom|OnQueryCancel
  (CallBack|OnQueryCancelFunc))

(event Custom|OnCreateMeshBased
  (params (ShapeType :type Integer) (count :type Integer))
  (CallBack|OnCreateMeshBasedFunc ShapeType count))

(event Custom|OnCreateRayMarchingOperation
  (params (OperationType :type RayMarchingOperationTypes%20Enum :default "NewEnumerator0"))
  (CallBack|OnCreateRayMarchingOperationFunc OperationType))

(event Custom|OnAdjustBigFlocking
  (CallBack|OnAdjustBigFlockingFunc))

(event Custom|OnCreateBigFlocking
  (params (ObjNum :type Integer))
  (CallBack|OnCreateBigFlockingFunc ObjNum))

(event Custom|OnAdjustAreaFog
  (CallBack|OnAdjustAreaFogFunc))

(event Custom|OnCreateSmallFlocking
  (params (objNum :type Integer))
  (CallBack|OnCreateSmallFlockingFunc objNum))

(event Custom|OnCreateAreaFog
  (CallBack|OnCreateAreaFogFunc))

(event Custom|OnChangeShapeMeshBased
  (params (shapeType :type Integer))
  (CallBack|OnChangeShapeMeshBasedFunc shapeType))

(event EventBeginPlay
  (Utilities|FlowControl|Sequence
    (:then_0
      (Variables|Default|SetCurrentTaskId 0)
      (Variables|Default|SetCurrentTaskStepId 0))
    (:then_1
      (bind _asfpspawn (Utilities|Casting|CastToFPSPawn (Game|Player|GetPlayerPawn 0)))
      (Utilities|FlowControl|Sequence
        (:then_0
          (EventDispatchers|BindEventtoOnCreateMeshBased (Variables|/Game/FPSMode/FPSPawn.FPSPawn_C|GetLeftController _asfpspawn) (delegate Custom|OnCreateMeshBased))
          (EventDispatchers|BindEventtoOnCreateRayMarching (Variables|/Game/FPSMode/FPSPawn.FPSPawn_C|GetLeftController _asfpspawn) (delegate Custom|OnCreateRayMarching))
          (EventDispatchers|BindEventtoOnCreateRayMarchingOperation (Variables|/Game/FPSMode/FPSPawn.FPSPawn_C|GetLeftController _asfpspawn) (delegate Custom|OnCreateRayMarchingOperation))
          (EventDispatchers|BindEventtoOnCreateBigFlocking (Variables|/Game/FPSMode/FPSPawn.FPSPawn_C|GetLeftController _asfpspawn) (delegate Custom|OnCreateBigFlocking))
          (EventDispatchers|BindEventtoOnCreateSmallFlocking (Variables|/Game/FPSMode/FPSPawn.FPSPawn_C|GetLeftController _asfpspawn) (delegate Custom|OnCreateSmallFlocking))
          (EventDispatchers|BindEventtoOnCreateAreaFog (Variables|/Game/FPSMode/FPSPawn.FPSPawn_C|GetLeftController _asfpspawn) (delegate Custom|OnCreateAreaFog))
          (EventDispatchers|BindEventtoOnChangeShapeMeshBased (Variables|/Game/FPSMode/FPSPawn.FPSPawn_C|GetLeftController _asfpspawn) (delegate Custom|OnChangeShapeMeshBased))
          (EventDispatchers|BindEventtoOnChangeShapeRayMarching (Variables|/Game/FPSMode/FPSPawn.FPSPawn_C|GetLeftController _asfpspawn) (delegate Custom|OnChangeShapeRayMarching))
          (EventDispatchers|BindEventtoOnChangeColorMeshBased (Variables|/Game/FPSMode/FPSPawn.FPSPawn_C|GetLeftController _asfpspawn) (delegate Custom|OnChangeColorMeshBased))
          (EventDispatchers|BindEventtoOnChangeColorRayMarching (Variables|/Game/FPSMode/FPSPawn.FPSPawn_C|GetLeftController _asfpspawn) (delegate Custom|OnChangeColorRayMarching))
          (EventDispatchers|BindEventtoOnScaleRayMarching (Variables|/Game/FPSMode/FPSPawn.FPSPawn_C|GetLeftController _asfpspawn) (delegate Custom|OnScaleRayMarching))
          (EventDispatchers|BindEventtoOnScaleCube (Variables|/Game/FPSMode/FPSPawn.FPSPawn_C|GetLeftController _asfpspawn) (delegate Custom|OnScaleCube))
          (EventDispatchers|BindEventtoOnAdjustSmallFlocking (Variables|/Game/FPSMode/FPSPawn.FPSPawn_C|GetLeftController _asfpspawn) (delegate Custom|OnAdjustSmallFlocking))
          (EventDispatchers|BindEventtoOnAdjustBigFlocking (Variables|/Game/FPSMode/FPSPawn.FPSPawn_C|GetLeftController _asfpspawn) (delegate Custom|OnAdjustBigFlocking))
          (EventDispatchers|BindEventtoOnAdjustAreaFog (Variables|/Game/FPSMode/FPSPawn.FPSPawn_C|GetLeftController _asfpspawn) (delegate Custom|OnAdjustAreaFog))
          (EventDispatchers|BindEventtoOnQuerySuccess (Variables|/Game/FPSMode/FPSPawn.FPSPawn_C|GetLeftController _asfpspawn) (delegate Custom|OnQuerySuccess))
          (EventDispatchers|BindEventtoOnQueryCancel (Variables|/Game/FPSMode/FPSPawn.FPSPawn_C|GetLeftController _asfpspawn) (delegate Custom|OnQueryCancel))
          (EventDispatchers|BindEventtoOnCreateFractal (Variables|/Game/FPSMode/FPSPawn.FPSPawn_C|GetLeftController _asfpspawn) (delegate Custom|OnCreateFractal)))
        (:then_1
          (EventDispatchers|BindEventtoTagsUpdate _asfpspawn (delegate Custom|OnTagsUpdate)))))))

(event Collision|EventActorBeginOverlap
  (params (OtherActor :type Actor%20Object%20Reference)))

(event EventTick
  (params (DeltaSeconds :type Float%20%28single-precision%29)))

(fn ConstructionScript)

(fn OnCreateMeshBasedFunc
  (params (ShapeType :type Integer) (count :type Integer))
  (Development|PrintString "OnCreateMeshBasedFunc")
  (bind (_issuccess _taskstepdata) (CallFunction|TryGetCurrentTaskStepData))
  (if _issuccess
    (if (Utilities|Enum|Equal(Enum) (.Type (Utilities|Struct|BreakTaskStepData _taskstepdata)) "CreateMeshBased")
      (CallFunction|UpdateTaskStep))))

(fn OnCreateRayMarchingFunc
  (params (GeometryType :type RayMarchingSingleShapeTypes%20Enum :default "NewEnumerator0") (count :type Integer))
  (Development|PrintString "OnCreateRayMarchingFunc")
  (bind (_issuccess _taskstepdata) (CallFunction|TryGetCurrentTaskStepData))
  (if _issuccess
    (if (Utilities|Enum|Equal(Enum) (.Type (Utilities|Struct|BreakTaskStepData _taskstepdata)) "CreateRayMarching")
      (CallFunction|UpdateTaskStep))))

(fn OnCreateRayMarchingOperationFunc
  (params (OperationType :type RayMarchingOperationTypes%20Enum :default "NewEnumerator0"))
  (Development|PrintString "OnCreateRayMarchingOperationFunc")
  (bind (_issuccess _taskstepdata) (CallFunction|TryGetCurrentTaskStepData))
  (if _issuccess
    (if (Utilities|Enum|Equal(Enum) (.Type (Utilities|Struct|BreakTaskStepData _taskstepdata)) "CreateRayMarchingOperation")
      (CallFunction|UpdateTaskStep))))

(fn OnCreateBigFlockingFunc
  (params (ObjNum :type Integer))
  (Development|PrintString "OnCreateBigFlockingFunc")
  (bind (_issuccess _taskstepdata) (CallFunction|TryGetCurrentTaskStepData))
  (if _issuccess
    (if (Utilities|Enum|Equal(Enum) (.Type (Utilities|Struct|BreakTaskStepData _taskstepdata)) "CreateBigFlocking")
      (CallFunction|UpdateTaskStep))))

(fn OnCreateSmallFlockingFunc
  (params (objNum :type Integer))
  (Development|PrintString "OnCreateSmallFlockingFunc")
  (bind (_issuccess _taskstepdata) (CallFunction|TryGetCurrentTaskStepData))
  (if _issuccess
    (if (Utilities|Enum|Equal(Enum) (.Type (Utilities|Struct|BreakTaskStepData _taskstepdata)) "CreateSmallFlocking")
      (CallFunction|UpdateTaskStep))))

(fn OnCreateAreaFogFunc
  (Development|PrintString "OnCreateAreaFogFunc")
  (bind (_issuccess _taskstepdata) (CallFunction|TryGetCurrentTaskStepData))
  (if _issuccess
    (if (Utilities|Enum|Equal(Enum) (.Type (Utilities|Struct|BreakTaskStepData _taskstepdata)) "CreateAreaFog")
      (CallFunction|UpdateTaskStep))))

(fn OnChangeShapeMeshBasedFunc
  (params (shapeType :type Integer))
  (Development|PrintString "OnChangeShapeMeshBased")
  (bind (_issuccess _taskstepdata) (CallFunction|TryGetCurrentTaskStepData))
  (if _issuccess
    (if (Utilities|Enum|Equal(Enum) (.Type (Utilities|Struct|BreakTaskStepData _taskstepdata)) "ChangeShapeMeshBased")
      (CallFunction|UpdateTaskStep))))

(fn OnChangeShapeRayMarchingFunc
  (params (GeometryType :type RayMarchingSingleShapeTypes%20Enum :default "NewEnumerator0"))
  (Development|PrintString "OnChangeShpaeRayMarching")
  (bind (_issuccess _taskstepdata) (CallFunction|TryGetCurrentTaskStepData))
  (if _issuccess
    (if (Utilities|Enum|Equal(Enum) (.Type (Utilities|Struct|BreakTaskStepData _taskstepdata)) "ChangeShapeRayMarching")
      (CallFunction|UpdateTaskStep))))

(fn OnChangeColorMeshBasedFunc
  (params (colorVector :type Vector))
  (Development|PrintString "OnChangeColorMeshBasedFunc")
  (bind (_issuccess _taskstepdata) (CallFunction|TryGetCurrentTaskStepData))
  (if _issuccess
    (if (Utilities|Enum|Equal(Enum) (.Type (Utilities|Struct|BreakTaskStepData _taskstepdata)) "ChangeColorMeshBased")
      (CallFunction|UpdateTaskStep))))

(fn OnChangeColorRayMarchingFunc
  (params (color :type Vector))
  (Development|PrintString "OnChangeColorRayMarchingFunc")
  (bind (_issuccess _taskstepdata) (CallFunction|TryGetCurrentTaskStepData))
  (if _issuccess
    (if (Utilities|Enum|Equal(Enum) (.Type (Utilities|Struct|BreakTaskStepData _taskstepdata)) "ChangeColorRayMarching")
      (CallFunction|UpdateTaskStep))))

(fn OnScaleRayMarchingFunc
  (Development|PrintString "OnScaleRayMarchingFunc")
  (bind (_issuccess _taskstepdata) (CallFunction|TryGetCurrentTaskStepData))
  (if _issuccess
    (if (Utilities|Enum|Equal(Enum) (.Type (Utilities|Struct|BreakTaskStepData _taskstepdata)) "ScaleRayMarching")
      (CallFunction|UpdateTaskStep))))

(fn OnScaleCubeFunc
  (Development|PrintString "OnScaleCubeFunc")
  (bind (_issuccess _taskstepdata) (CallFunction|TryGetCurrentTaskStepData))
  (if _issuccess
    (if (Utilities|Enum|Equal(Enum) (.Type (Utilities|Struct|BreakTaskStepData _taskstepdata)) "ScaleCube")
      (CallFunction|UpdateTaskStep))))

(fn OnQuerySuccessFunc
  (Development|PrintString "OnQuerySuccessFunc")
  (bind (_issuccess _taskstepdata) (CallFunction|TryGetCurrentTaskStepData))
  (if _issuccess
    (if (Utilities|Enum|Equal(Enum) (.Type (Utilities|Struct|BreakTaskStepData _taskstepdata)) "QuerySuccessUpdate")
      (CallFunction|UpdateTaskStep))))

(fn OnQueryCancelFunc
  (Development|PrintString "OnQueryCancelFunc")
  (bind (_issuccess _taskstepdata) (CallFunction|TryGetCurrentTaskStepData))
  (if _issuccess
    (if (Utilities|Enum|Equal(Enum) (.Type (Utilities|Struct|BreakTaskStepData _taskstepdata)) "QueryCancelUpdate")
      (CallFunction|UpdateTaskStep))))

(fn OnTagsUpdateFunc
  (Development|PrintString "OnTagsUpdateFunc")
  (bind (_issuccess _taskstepdata) (CallFunction|TryGetCurrentTaskStepData))
  (if _issuccess
    (if (Utilities|Enum|Equal(Enum) (.Type (Utilities|Struct|BreakTaskStepData _taskstepdata)) "TagsUpdate")
      (CallFunction|UpdateTaskStep))))

(fn UpdateTaskStep
  (bind _isfinishalltasks (CallFunction|IsFinishAllTask))
  (if (not _isfinishalltasks)
    (if (< (+ (Variables|Default|GetCurrentTaskStepId) 1) (Utilities|Array|Length (.TaskStepList (Utilities|Struct|BreakTaskData (Utilities|Array|Get(acopy) (Variables|/Script/MyVRDemo.TaskDataAsset|GetTaskDataList (Variables|Default|GetTaskAssetData)) (Variables|Default|GetCurrentTaskId))))))
      (bind _output_get (Variables|Default|SetCurrentTaskStepId (+ (Variables|Default|GetCurrentTaskStepId) 1)))
      (Development|PrintString (Utilities|String|Append (Utilities|String|ToString(Integer) _output_get) " current task step"))
      (else
        (Variables|Default|SetCurrentTaskStepId 0)
        (bind _output_get_2 (Variables|Default|SetCurrentTaskId (+ (Variables|Default|GetCurrentTaskId) 1)))
        (Development|PrintString (Utilities|String|Append (Utilities|String|ToString(Integer) _output_get_2) " current Task Id"))
        (bind _isfinishalltasks_2 (CallFunction|IsFinishAllTask))
        (if _isfinishalltasks_2
          (Development|PrintString "Finish All Task!!!!!!"))))
    (Default|CallTaskUpdate)))

(fn IsFinishAllTask
  (if (< (Variables|Default|GetCurrentTaskId) (Utilities|Array|Length (Variables|/Script/MyVRDemo.TaskDataAsset|GetTaskDataList (Variables|Default|GetTaskAssetData))))
    (return false)
    (else
      (return true))))

(fn TryGetCurrentTaskStepData
  (bind _currenttaskstepid (Variables|Default|GetCurrentTaskStepId))
  (bind _taskassetdata (Variables|Default|GetTaskAssetData))
  (bind _currenttaskid (Variables|Default|GetCurrentTaskId))
  (bind _taskdatalist (Variables|/Script/MyVRDemo.TaskDataAsset|GetTaskDataList _taskassetdata))
  (bind _output (Utilities|Array|Get(acopy) _taskdatalist _currenttaskid))
  (bind _tasksteplist (Utilities|Struct|BreakTaskData _output))
  (bind _isfinishalltasks (CallFunction|IsFinishAllTask))
  (if _isfinishalltasks
    (return false "" "")
    (elif (< _currenttaskstepid (Utilities|Array|Length _tasksteplist))
      (return true (Utilities|Array|Get(acopy) _tasksteplist _currenttaskstepid) _output)
      (else
        (return false "" "")))))

(fn OnAdjustSmallFlockingFunc
  (Development|PrintString "OnAdjustSmallFlockingFunc")
  (bind (_issuccess _taskstepdata) (CallFunction|TryGetCurrentTaskStepData))
  (if _issuccess
    (if (Utilities|Enum|Equal(Enum) (.Type (Utilities|Struct|BreakTaskStepData _taskstepdata)) "AdjustSmallFlocking")
      (CallFunction|UpdateTaskStep))))

(fn OnAdjustBigFlockingFunc
  (Development|PrintString "OnAdjustBigFlockingFunc")
  (bind (_issuccess _taskstepdata) (CallFunction|TryGetCurrentTaskStepData))
  (if _issuccess
    (if (Utilities|Enum|Equal(Enum) (.Type (Utilities|Struct|BreakTaskStepData _taskstepdata)) "AdjustBigFlocking")
      (CallFunction|UpdateTaskStep))))

(fn OnAdjustAreaFogFunc
  (Development|PrintString "OnAdjustAreaFogFunc")
  (bind (_issuccess _taskstepdata) (CallFunction|TryGetCurrentTaskStepData))
  (if _issuccess
    (if (Utilities|Enum|Equal(Enum) (.Type (Utilities|Struct|BreakTaskStepData _taskstepdata)) "AdjustAreaFog")
      (CallFunction|UpdateTaskStep))))

(fn OnCreateFractalFunc
  (Development|PrintString "OnCreateFractalFunc")
  (bind (_issuccess _taskstepdata) (CallFunction|TryGetCurrentTaskStepData))
  (if _issuccess
    (if (Utilities|Enum|Equal(Enum) (.Type (Utilities|Struct|BreakTaskStepData _taskstepdata)) "CreateFractal")
      (CallFunction|UpdateTaskStep))))