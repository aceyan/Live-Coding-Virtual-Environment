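; BP_BigFlocking is a flocking controller that spawns and tunes a MyCSTestActor for a configurable number of objects.
; On BeginPlay it spawns that actor with the object count and minimum range, then attaches it to itself.
; Each Tick it copies its separation, cohesion and alignment force scalers into the spawned actor, which leaves the flock simulation outside this Blueprint.
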(event EventBeginPlay
  (bind _objectnum (Variables|flocking|GetObjectNum))
  (bind _returnvalue (Game|SpawnActorfromClass "/Game/Flocking/MyCSTestActor.MyCSTestActor_C" (Math|Transform|MakeTransform "0, 0, 0" "0, 0, 0" "1,1,1") "AlwaysSpawn" 0 _objectnum "1000.000000,1000.000000,1000.000000" "-1000.000000,-1000.000000,20.000000" 0.01 5.0 (Math|Conversions|ToFloat(Integer) _objectnum) 0))
  (bind _output_get (Variables|flocking|SetMyCSTestActor _returnvalue))
  (Transformation|AttachActorToActor _output_get self "None" "KeepRelative" "KeepRelative" "KeepRelative" true))

(event Collision|EventActorBeginOverlap
  (params (OtherActor :type Actor%20Object%20Reference)))

(event EventTick
  (params (DeltaSeconds :type Float%20%28single-precision%29))
  (bind _mycstestactor (Variables|flocking|GetMyCSTestActor))
  (Utilities|IsValid _mycstestactor
    (:Is%20Valid
      (Variables|/Script/MyVRDemo.CSTestActor|SetSeparationForceScaler _mycstestactor (Variables|flocking|GetSeparationForceScaler))
      (Variables|/Script/MyVRDemo.CSTestActor|SetCohesionForceScaler _mycstestactor (Variables|flocking|GetCohesionForceScaler))
      (Variables|/Script/MyVRDemo.CSTestActor|SetAlignForceScaler _mycstestactor (Variables|flocking|GetAlignForceScaler)))))

(fn ConstructionScript)