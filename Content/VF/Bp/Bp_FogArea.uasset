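; Bp_FogArea is a resizable fog area actor built on a static mesh component.
; On BeginPlay it creates a dynamic instance of VF_DOF_Blend_Inst and assigns it to the mesh, without setting any parameters.
; Every Tick it scales the actor from its length, width and height variables divided by 100, and overrides world Z to half the height plus a small offset, keeping X and Y.
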(event EventBeginPlay
  (bind _returnvalue (Rendering|Material|CreateDynamicMaterialInstance "/Game/VF/Mat_DOF/VF_DOF_Blend_Inst.VF_DOF_Blend_Inst" "None" :!class /Script/Engine.KismetMaterialLibrary))
  (Rendering|Material|SetMaterial (Variables|Debug|GetStaticMeshComponent) 0 _returnvalue))

(event Collision|EventActorBeginOverlap
  (params (OtherActor :type Actor%20Object%20Reference)))

(event EventTick
  (params (DeltaSeconds :type Float%20%28single-precision%29))
  (bind _returnvalue (Transformation|GetActorLocation))
  (Transformation|SetActorLocation (Math|Vector|MakeVector (.x _returnvalue) (.y _returnvalue) (+ (/ (Variables|Default|GetHeightAreaFog) 2.0) 2e+01)) false false)
  (Transformation|SetActorScale3D (Math|Vector|MakeVector (/ (Variables|Default|GetLengthAreaFog) 1e+02) (/ (Variables|Default|GetWidthAreaFog) 1e+02) (/ (Variables|Default|GetHeightAreaFog) 1e+02))))

(fn ConstructionScript)